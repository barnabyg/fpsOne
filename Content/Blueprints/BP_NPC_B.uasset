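; NPC actor that switches between looping idle and talk animations when the player's interaction component targets it for dialogue.
; Tick delays each switch until playback is in an early or late time window, carrying the truncated position into the new animation.
; On other ticks it eases yaw slightly toward a nearby player, clamped around a fixed 180-degree facing.
; The construction script hides the proxy body and head.
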(event `self.ReceiveTick`
  (params (DeltaSeconds :type "Float (single-precision)"))
  (bind _returnvalue (`GameplayStatics.GetPlayerPawn` 0))
  (bind _charactervisual (`self.CharacterVisual`))
  (bind _returnvalue_2 (`self.GetComponentByClass` _returnvalue "/Game/Blueprints/BPC_Interaction.BPC_Interaction_C"))
  (bind _returnvalue_3 (`SkeletalMeshComponent.GetPosition` _charactervisual))
  (bind _returnvalue_4 (== (`/Game/Blueprints/BPC_Interaction.DialogueActor` _returnvalue_2) self))
  (if (`KismetSystemLibrary.IsValid` _returnvalue_2)
    (if (and (!= _returnvalue_4 (`self.TalkPlaying`)) (or (<= _returnvalue_3 1.0) (>= _returnvalue_3 4.0)))
      (set `self.TransitionPhase` (`KismetMathLibrary.FTrunc` _returnvalue_3))
      (set `self.TalkPlaying` _returnvalue_4)
      (if _returnvalue_4
        (`SkeletalMeshComponent.PlayAnimation` _charactervisual "/Game/Characters/NPC_B/B_Talk.B_Talk" true)
        (`SkeletalMeshComponent.SetPosition` _charactervisual (`KismetMathLibrary.Conv_IntToDouble` (`self.TransitionPhase`)) false)
        (else
          (`SkeletalMeshComponent.PlayAnimation` _charactervisual "/Game/Characters/NPC_B/B_Idle.B_Idle" true)
          (`SkeletalMeshComponent.SetPosition` _charactervisual (`KismetMathLibrary.Conv_IntToDouble` (`self.TransitionPhase`)) false)))
      (else
        (`self.K2_SetActorRotation` (`KismetMathLibrary.RInterpTo` (`self.K2_GetActorRotation`) (`KismetMathLibrary.MakeRotator` 0.0 0.0 (+ (`KismetMathLibrary.SelectFloat` (`KismetMathLibrary.FClamp` (.yaw (`KismetMathLibrary.NormalizedDeltaRotator` (`KismetMathLibrary.FindLookAtRotation` (`self.K2_GetActorLocation`) (`self.K2_GetActorLocation` _returnvalue)))) -12.0 12.0) 0.0 (< (`self.GetDistanceTo` _returnvalue) 300.0)) 180.0)) DeltaSeconds 1.2))))))

(fn `UserConstructionScript`
  (`SceneComponent.SetVisibility` (`self.ProxyBody`) false false)
  (`SceneComponent.SetVisibility` (`self.ProxyHead`) false false))