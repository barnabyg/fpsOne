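; BPC_Interaction is a component that lets the player find and trigger objects carrying a BPC_Interactable component.
; ScanForInteractionFocus runs a short Visibility line trace from the camera manager, caching an available interactable and its prompt, or clearing both otherwise.
; TryInteract rechecks the cached focus's validity and availability, then calls its RequestInteraction.
; BeginPlay and Tick are unused, so both functions rely on external callers.
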(fn `ScanForInteractionFocus`
  (bind _returnvalue (`GameplayStatics.GetPlayerCameraManager` 0))
  (bind _returnvalue_2 (`Actor.K2_GetActorLocation` _returnvalue))
  (bind (_outhit _returnvalue_3) (`KismetSystemLibrary.LineTraceSingle` _returnvalue_2 (+ _returnvalue_2 (* (`Actor.GetActorForwardVector` _returnvalue) (250.0 250.0 250.0))) "TraceTypeQuery1"))
  (if _returnvalue_3
    (bind _returnvalue_4 (`Actor.GetComponentByClass` (`.HitActor` (`GameplayStatics.BreakHitResult` _outhit)) "/Game/Blueprints/BPC_Interactable.BPC_Interactable_C"))
    (if (`KismetSystemLibrary.IsValid` _returnvalue_4)
      (if (`/Game/Blueprints/BPC_Interactable.InteractionAvailable` _returnvalue_4)
        (set `self.CurrentFocus` _returnvalue_4)
        (set `self.CurrentPrompt` (`/Game/Blueprints/BPC_Interactable.InteractionPrompt` _returnvalue_4))
        (else
          (set `self.CurrentFocus` null)
          (set `self.CurrentPrompt` "")))
      (else
        (set `self.CurrentFocus` null)
        (set `self.CurrentPrompt` "")))
    (else
      (set `self.CurrentFocus` null)
      (set `self.CurrentPrompt` ""))))

(fn `TryInteract`
  (bind _currentfocus (`self.CurrentFocus`))
  (if (`KismetSystemLibrary.IsValid` _currentfocus)
    (if (`/Game/Blueprints/BPC_Interactable.InteractionAvailable` _currentfocus)
      (`/Game/Blueprints/BPC_Interactable.RequestInteraction` _currentfocus))))