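; BP_Player is the player pawn, with axis-driven movement, look controls and interaction with the world.
; Movement follows the actor's forward and right vectors, while Turn and LookUp feed controller yaw and pitch.
; An Interaction component scans for focus and refreshes its presentation every Tick, and the Interact action asks it to attempt an interaction.
; The Exit action quits the game immediately.
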(event `InputAxis|MoveForward`
  (params (AxisValue :type "Float (single-precision)"))
  (`self.AddMovementInput` (`self.GetActorForwardVector`) AxisValue))

(event `InputAxis|MoveRight`
  (params (AxisValue :type "Float (single-precision)"))
  (`self.AddMovementInput` (`self.GetActorRightVector`) AxisValue))

(event `InputAxis|Turn`
  (params (AxisValue :type "Float (single-precision)"))
  (`self.AddControllerYawInput` AxisValue))

(event `InputAxis|LookUp`
  (params (AxisValue :type "Float (single-precision)"))
  (`self.AddControllerPitchInput` AxisValue))

(event `InputAction|Exit`
  (params (Key :type "Key Structure"))
  (:`Pressed`
    (`KismetSystemLibrary.QuitGame` null "Quit")))

(event `self.ReceiveTick`
  (params (DeltaSeconds :type "Float (single-precision)"))
  (bind _interaction (`self.Interaction`))
  (`/Game/Blueprints/BPC_Interaction.ScanForInteractionFocus` _interaction)
  (`/Game/Blueprints/BPC_Interaction.RefreshPresentation` _interaction))

(event `InputAction|Interact`
  (params (Key :type "Key Structure"))
  (:`Pressed`
    (`/Game/Blueprints/BPC_Interaction.TryInteract` (`self.Interaction`))))

(fn `UserConstructionScript`)