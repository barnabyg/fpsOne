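; Hinged door actor that the player toggles open and closed through an Interactable component.
; InteractionZone blocks only Visibility for queries, and each interaction request eases the Hinge between closed and 90-degree yaw using MoveComponentTo.
; IsMoving and the availability flag block input mid-swing, then the prompt switches between Open and Close.
; DoorLeaf stops blocking pawns when movement starts and blocks them again only once fully closed.
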(event `self.ReceiveBeginPlay`
  (bind _interactable (`self.Interactable`))
  (bind _interactionzone (`self.InteractionZone`))
  (`PrimitiveComponent.SetCollisionEnabled` _interactionzone "QueryOnly")
  (`PrimitiveComponent.SetCollisionResponseToAllChannels` _interactionzone "ECR_Ignore")
  (`PrimitiveComponent.SetCollisionResponseToChannel` _interactionzone "ECC_Visibility" "ECR_Block")
  (set `/Game/Blueprints/BPC_Interactable.InteractionPrompt` "E — Open" _interactable)
  (set `/Game/Blueprints/BPC_Interactable.InteractionAvailable` true _interactable)
  (add `/Game/Blueprints/BPC_DoorInteractable.InteractionRequested` _interactable (delegate `HandleInteractionRequest`)))

(event `HandleInteractionRequest`
  (bind _doorleaf (`self.DoorLeaf`))
  (bind _interactable (`self.Interactable`))
  (bind _doorleaf_2 (`self.DoorLeaf`))
  (bind _interactable_2 (`self.Interactable`))
  (if (`self.IsMoving`)
    _
    (elif (`self.IsOpen`)
      (set `self.IsMoving` true)
      (set `/Game/Blueprints/BPC_Interactable.InteractionAvailable` false _interactable_2)
      (`PrimitiveComponent.SetCollisionEnabled` _doorleaf_2 "QueryOnly")
      (`PrimitiveComponent.SetCollisionResponseToChannel` _doorleaf_2 "ECC_Pawn" "ECR_Ignore")
      (`KismetSystemLibrary.MoveComponentTo` (`self.Hinge`) (0.0 50.0 0.0) (struct) true true 0.75 true)
      (set `self.IsOpen` false)
      (`PrimitiveComponent.SetCollisionEnabled` _doorleaf_2 "QueryAndPhysics")
      (`PrimitiveComponent.SetCollisionResponseToChannel` _doorleaf_2 "ECC_Pawn" "ECR_Block")
      (set `/Game/Blueprints/BPC_Interactable.InteractionPrompt` "E — Open" _interactable_2)
      (set `/Game/Blueprints/BPC_Interactable.InteractionAvailable` true _interactable_2)
      (set `self.IsMoving` false)
      (else
        (set `self.IsMoving` true)
        (set `/Game/Blueprints/BPC_Interactable.InteractionAvailable` false _interactable)
        (`PrimitiveComponent.SetCollisionEnabled` _doorleaf "QueryOnly")
        (`PrimitiveComponent.SetCollisionResponseToChannel` _doorleaf "ECC_Pawn" "ECR_Ignore")
        (`KismetSystemLibrary.MoveComponentTo` (`self.Hinge`) (0.0 50.0 0.0) (struct :`Yaw` 90) true true 0.75 true)
        (set `self.IsOpen` true)
        (set `/Game/Blueprints/BPC_Interactable.InteractionPrompt` "E — Close" _interactable)
        (set `/Game/Blueprints/BPC_Interactable.InteractionAvailable` true _interactable)
        (set `self.IsMoving` false)))))

(fn `UserConstructionScript`)